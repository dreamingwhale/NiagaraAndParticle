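; Traffic light actor that demonstrates RepNotify variable replication by changing which light it shows.
; On BeginPlay, only the authority runs an endless delay loop that sets StreetlightScalar to yellow, green, then red, with a random wait before each cycle.
; OnRep_StreetlightScalar pushes the value into a dynamic material instance, created on the mesh in the construction script, to update the visual.
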(event EventBeginPlay
  (Networking|SwitchHasAuthority :!label _label
    (:Authority
      (Utilities|FlowControl|Delay (Math|Random|RandomFloatinRange 2.0 5.0))
      (Variables|Default|SetStreetlightScalar (Variables|Default|GetYellowScalar))
      (Utilities|FlowControl|Delay 1.0)
      (Variables|Default|SetStreetlightScalar (Variables|Default|GetGreenScalar))
      (Utilities|FlowControl|Delay 1.0)
      (Variables|Default|SetStreetlightScalar (Variables|Default|GetRedScalar))
      (goto _label))))

(event Collision|EventActorBeginOverlap
  (params (OtherActor :type Actor%20Object%20Reference)))

(event EventTick
  (params (DeltaSeconds :type Float%20%28single-precision%29)))

(fn ConstructionScript
  (bind _returnvalue (Rendering|Material|CreateDynamicMaterialInstance (Variables|Default|GetSM_Traffic_Light) 1 0 "None" :!class /Script/Engine.PrimitiveComponent))
  (Variables|Default|SetMI_Light _returnvalue))

(fn OnRepStreetlightScalar
  (Rendering|Material|SetScalarParameterValue (Variables|Default|GetMI_Light) (Variables|Default|GetStreetlightScalarParamName) (Variables|Default|GetStreetlightScalar) :!class /Script/Engine.MaterialInstanceDynamic))