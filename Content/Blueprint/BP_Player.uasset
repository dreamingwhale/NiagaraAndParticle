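; BP_Player is a player actor that moves with axis input and fires bullets on left mouse click.
; Movement adds unswept world offsets along the camera manager's forward and right vectors, scaled by input with no delta time.
; Firing spawns BP_Bullet at a fixed world-X offset from the player and pushes its sphere with a world-X impulse, regardless of facing.
; An HP RepNotify function exists but is empty.
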(event EventBeginPlay)

(event Collision|EventActorBeginOverlap
  (params (OtherActor :type Actor%20Object%20Reference)))

(event EventTick
  (params (DeltaSeconds :type Float%20%28single-precision%29)))

(event Input|AxisEvents|InputAxisMoveForward
  (params (AxisValue :type Float%20%28single-precision%29))
  (Transformation|AddActorWorldOffset (* (Transformation|GetActorForwardVector (Game|GetPlayerCameraManager 0)) (* AxisValue 1e+01))))

(event Input|AxisEvents|InputAxisMoveRight
  (params (AxisValue :type Float%20%28single-precision%29))
  (Transformation|AddActorWorldOffset (* (Transformation|GetActorRightVector (Game|GetPlayerCameraManager 0)) (* AxisValue 1e+01))))

(event Input|MouseEvents|LeftMouseButton
  (params (Key :type Key%20Structure :default "None"))
  (bind _returnvalue (Transformation|GetActorTransform))
  (:Pressed
    (bind _returnvalue_2 (Game|SpawnActorfromClass "/Game/Blueprint/BP_Bullet.BP_Bullet_C" (Math|Transform|MakeTransform (+ (.location _returnvalue) "50.000000,0.000000,0.000000") (.rotation _returnvalue) (.scale _returnvalue)) "Undefined" "MultiplyWithRoot" 0 0))
    (Physics|AddImpulse (Variables|/Game/Blueprint/BP_Bullet.BP_Bullet_C|GetSphere _returnvalue_2) "100.000000,0.000000,0.000000" "None" false)))

(fn ConstructionScript)

(fn OnRepHP)