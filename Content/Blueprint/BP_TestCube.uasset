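; BP_TestCube is a clickable cube that reacts more intensely with each click and eventually explodes.
; On BeginPlay it creates a dynamic material instance on the cube for runtime color changes.
; Each click raises a counter that drives red emissive intensity and click sound pitch.
; Once the counter exceeds five, the next click destroys the actor after a brief delay and spawns an explosion at its XY position.
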(event OnClicked(Cube)
  (params (TouchedComponent :type Primitive%20Component%20Object%20Reference) (ButtonPressed :type Key%20Structure :default "None"))
  (bind _returnvalue (Transformation|GetActorLocation))
  (if (<= (Variables|Default|GetOnClickedNum) 5)
    (Variables|Default|SetOnClickedNum (+ (Variables|Default|GetOnClickedNum) 1))
    (Rendering|Material|SetVectorParameterValue (Variables|Default|GetCubeParameter) "EmissiveColor" (Utilities|Struct|MakeLinearColor (Math|Conversions|ToFloat(Integer) (* (Variables|Default|GetOnClickedNum) 100)) 0.0 0.0 1.0) :!class /Script/Engine.MaterialInstanceDynamic)
    (Audio|PlaySound2D "/Engine/VREditor/Sounds/UI/Click_on_Button.Click_on_Button" 2.0 (Math|Conversions|ToFloat(Integer) (* (Variables|Default|GetOnClickedNum) 1)) 0.0 0 0)
    (else
      (Utilities|FlowControl|Delay 0.2)
      (Actor|DestroyActor)
      (Effects|SpawnEmitteratLocation "/Game/StarterContent/Particles/P_Explosion.P_Explosion" (Math|Vector|MakeVector (.x _returnvalue) (.y _returnvalue) 1e+01)))))

(event EventBeginPlay
  (bind _returnvalue (Rendering|Material|CreateDynamicMaterialInstance (Variables|Default|GetCube) 0 0 "" :!class /Script/Engine.PrimitiveComponent))
  (Variables|Default|SetCubeParameter _returnvalue))

(event Collision|EventActorBeginOverlap
  (params (OtherActor :type Actor%20Object%20Reference)))

(event EventTick
  (params (DeltaSeconds :type Float%20%28single-precision%29)))

(fn ConstructionScript)